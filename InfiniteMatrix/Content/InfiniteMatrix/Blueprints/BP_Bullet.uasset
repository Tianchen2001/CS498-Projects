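; BP_Bullet is a projectile actor that moves only while the game mode is GM_Tutorial.
; Each Tick offsets it along world X by ForwardSpeed scaled by delta time, with sweep enabled, and destroys it once it is one second old.
; SetSpeed sets ForwardSpeed; the file contains no hit or damage handling, and a failed game mode cast skips both movement and destruction.
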(event EventTick
  (params (DeltaSeconds :type Float%20%28single-precision%29))
  (Utilities|Casting|CastToGM_Tutorial (Game|GetGameMode))
  (Transformation|AddActorWorldOffset (Math|Vector|MakeVector (* DeltaSeconds (Variables|Default|GetForwardSpeed)) 0.0 0.0) true)
  (if (>= (Actor|GetGameTimeSinceCreation) 1.0)
    (Actor|DestroyActor)))

(fn ConstructionScript)

(fn SetSpeed
  (params (Speed :type Float%20%28single-precision%29))
  (Variables|Default|SetForwardSpeed Speed))