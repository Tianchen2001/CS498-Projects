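; GM_Tutorial is the tutorial game mode Blueprint that tracks the current health and score and shows them on the HUD.
; On BeginPlay it creates a WBP_HUD widget, stores it and adds it to the viewport.
; Custom events add to score or health, set health directly, or reset to full health and zero score, each pushing the new values straight into the widget without clamping.
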(event Custom|Reset
  (bind _hud (Variables|Default|GetHUD))
  (bind _output_get (Variables|Default|SetCurrentHealth (Variables|Default|GetMaxHealth)))
  (Variables|/Game/InfiniteMatrix/UI/WBP_HUD.WBP_HUD_C|SetHealth _hud _output_get)
  (Variables|/Game/InfiniteMatrix/UI/WBP_HUD.WBP_HUD_C|SetScore _hud 0)
  (Variables|Default|SetCurrentScore 0))

(event Custom|UpdateScore
  (params (Score :type Integer))
  (Variables|Default|SetCurrentScore (+ Score (Variables|Default|GetCurrentScore)))
  (Variables|/Game/InfiniteMatrix/UI/WBP_HUD.WBP_HUD_C|SetScore (Variables|Default|GetHUD) (Variables|Default|GetCurrentScore)))

(event Custom|UpdateHealth
  (params (Health :type Integer))
  (Variables|Default|SetCurrentHealth (+ Health (Variables|Default|GetCurrentHealth)))
  (Variables|/Game/InfiniteMatrix/UI/WBP_HUD.WBP_HUD_C|SetHealth (Variables|Default|GetHUD) (Variables|Default|GetCurrentHealth)))

(event Custom|SetHealth
  (params (Health :type Integer))
  (Variables|Default|SetCurrentHealth Health)
  (Variables|/Game/InfiniteMatrix/UI/WBP_HUD.WBP_HUD_C|SetHealth (Variables|Default|GetHUD) (Variables|Default|GetCurrentHealth)))

(event EventBeginPlay
  (bind _returnvalue (UserInterface|CreateWidget "/Game/InfiniteMatrix/UI/WBP_HUD.WBP_HUD_C"))
  (bind _output_get (Variables|Default|SetHUD _returnvalue))
  (UserInterface|Viewport|AddtoViewport _output_get 0))

(fn ConstructionScript)