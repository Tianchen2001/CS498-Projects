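; BP_Enemy is an enemy actor that damages the player on contact and awards score when shot.
; Player overlap on the Enemy component plays a camera shake, lowers health through GM_Tutorial and destroys the enemy, marking the player dead and showing restart at zero health.
; A BP_Bullet overlap destroys both actors and adds score through GM_Tutorial.
; A separate TriggerZone destroys the enemy on player overlap without changing health or score.
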(event OnComponentBeginOverlap(Enemy)
  (params (OverlappedComponent :type Primitive%20Component%20Object%20Reference) (OtherActor :type Actor%20Object%20Reference) (OtherComp :type Primitive%20Component%20Object%20Reference) (OtherBodyIndex :type Integer) (bFromSweep :type Boolean) (SweepResult :type Hit%20Result%20Structure%20%28by%20ref%29))
  (bind _asbp_player (Utilities|Casting|CastToBP_Player OtherActor)
    (:then
      (Camera|PlayWorldCameraShake "/Game/InfiniteMatrix/Blueprints/Camerashake.Camerashake_C" (Transformation|GetWorldLocation (Variables|/Game/InfiniteMatrix/Blueprints/BP_Player.BP_Player_C|GetCamera _asbp_player)) 1e+02 1e+03)
      (bind _asgm_tutorial (Utilities|Casting|CastToGM_Tutorial (Game|GetGameMode)))
      (Default|UpdateHealth _asgm_tutorial -1)
      (Actor|DestroyActor)
      (if (<= (Variables|/Game/InfiniteMatrix/Blueprints/GM_Tutorial.GM_Tutorial_C|GetCurrentHealth _asgm_tutorial) 0)
        (Variables|/Game/InfiniteMatrix/Blueprints/BP_Player.BP_Player_C|SetIsDead _asbp_player true)
        (Default|DisplayRestart _asbp_player)))
    (:CastFailed
      (bind _asbp_bullet (Utilities|Casting|CastToBP_Bullet OtherActor))
      (Actor|DestroyActor _asbp_bullet)
      (bind _asgm_tutorial_2 (Utilities|Casting|CastToGM_Tutorial (Game|GetGameMode)))
      (Default|UpdateScore _asgm_tutorial_2 1)
      (Actor|DestroyActor))))

(event OnComponentBeginOverlap(TriggerZone)
  (params (OverlappedComponent :type Primitive%20Component%20Object%20Reference) (OtherActor :type Actor%20Object%20Reference) (OtherComp :type Primitive%20Component%20Object%20Reference) (OtherBodyIndex :type Integer) (bFromSweep :type Boolean) (SweepResult :type Hit%20Result%20Structure%20%28by%20ref%29))
  (Utilities|Casting|CastToBP_Player OtherActor)
  (Actor|DestroyActor))

(fn ConstructionScript)